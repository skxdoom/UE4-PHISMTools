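; PHISM tool Blueprint that procedurally fills a 3D grid with randomly picked HISM mesh instances from the construction script.
; Each cell, spaced by a set distance plus optional mesh size, gets random location jitter and a line trace for placement.
; Cells passing the trace and spawn-chance roll add an instance with pivot and vertical offsets, trace-aligned or custom rotation plus random variation, and scale.
; A shared random stream drives the randomization.
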(event EventBeginPlay)

(event Collision|EventActorBeginOverlap
  (params (OtherActor :type Actor%20Object%20Reference)))

(event EventTick
  (params (DeltaSeconds :type Float%20%28single-precision%29)))

(fn ConstructionScript
  (|CallParentFunction)
  (CallFunction|SpawnInstances))

(fn SpawnInstances
  (bind _add_mesh_size_to_spacing (Variables|Placement|GetAdd%20Mesh%20Size%20to%20Spacing))
  (bind _spacing (Variables|Placement|GetSpacing))
  (bind _instance_box_extent_temp (Variables|Default|GetInstance%20Box%20Extent%20Temp))
  (bind _returnvalue (* _instance_box_extent_temp 2.0))
  (bind _returnvalue_2 (select _add_mesh_size_to_spacing _returnvalue "0, 0, 0"))
  (bind _returnvalue_3 (+ _returnvalue_2 _spacing))
  (bind (_x _y _z) (Math|Vector|BreakVector _returnvalue_3))
  ;[1 1 1] Main Loop
  (for _index (range 0 (- (Variables|Meshes|GetMeshes%20X) 1))
    (for _index_2 (range 0 (- (Variables|Meshes|GetMeshes%20Y) 1))
      (for _index_3 (range 0 (- (Variables|Meshes|GetMeshes%20Z) 1))
        (CallFunction|SetInstanceTemporalValues (Utilities|GetRandomHISM (Variables|Default|GetHISM%20Array) (Variables|Default|GetHISM%20Array%20Length) (Variables|Default|GetRandomStream)))
        (bind (_location_output _align_rotation_output _canspawn) (CallFunction|LineTracingforPlacement (Utilities|AddRandomLocation (Math|Vector|MakeVector (* _index _x) (* _index_2 _y) (* _index_3 _z)) (Variables|Placement|GetAdd%20Random%20Location) (Variables|Default|GetRandomStream)) (Variables|Default|GetCollision%20Tracing%20Distance)))
        (if _canspawn
          (if (Utilities|GetRandomChance (Variables|Placement|GetSpawn%20Chance) (Variables|Default|GetRandomStream))
            (Components|InstancedStaticMesh|AddInstance (Variables|Default|GetInstance%20Temp) (Math|Transform|MakeTransform (Utilities|AddVerticalLocation (select (Variables|Default|GetPivot%20Point%20At%20Zero) _location_output (+ _location_output (Math|Vector|MakeVector 0.0 0.0 (.Z (Math|Vector|BreakVector (Variables|Default|GetInstance%20Box%20Extent%20Temp)))))) (Variables|Default|GetAdd%20Vertical%20Location)) (Utilities|AddRandomRotation (Math|Rotator|SelectRotator (Variables|Placement|GetAdd%20Custom%20Rotation) _align_rotation_output (Variables|Placement|GetCustom%20Rotation)) (Variables|Default|GetAdd%20Random%20Rotation) (Variables|Default|GetRandomStream)) (Variables|Default|GetInstance%20Scale%20Temp)))))))))