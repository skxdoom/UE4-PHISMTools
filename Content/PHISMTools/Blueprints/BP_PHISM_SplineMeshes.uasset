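; PHISM Tools Blueprint that scatters instanced meshes along a spline at construction time.
; The construction script steps along the spline by Spacing, rolls a spawn chance and adds an instance to a random HISM from an array.
; Each transform combines spline-aligned or custom rotation with offsets and random location, rotation and per-axis scale from a random stream.
; RandomizeSpacing varies only the loop count, using unseeded randomness, not the step distance.
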(event EventBeginPlay)

(event Collision|EventActorBeginOverlap
  (params (OtherActor :type Actor%20Object%20Reference)))

(event EventTick
  (params (DeltaSeconds :type Float%20%28single-precision%29)))

(fn ConstructionScript
  (|CallParentFunction)
  (CallFunction|SpawnInstancesbySpacing) ; Spawn Instances with user defined parameters
)

(fn SpawnInstancesbySpacing
  (bind _randomstream (Variables|Default|GetRandomStream))
  (bind _scale_min (Variables|Default|GetScale%20Min))
  (bind _scale_max (Variables|Default|GetScale%20Max))
  (bind _spline (Variables|Default|GetSpline))
  (bind _randomize_spacing (Variables|Placement|GetRandomize%20Spacing))
  (bind _scale_output (Utilities|GetRandomScale _scale_min _scale_max _randomstream))
  (for _index (range 0 (.ReturnValue (Math|Float|Division(WholeandRemainder) (Spline|GetSplineLength (Variables|Default|GetSpline)) (+ (Variables|Placement|GetSpacing) (Math|Random|RandomFloatinRange (* _randomize_spacing -1.0) _randomize_spacing)))))
    (if (Utilities|GetRandomChance (Variables|Placement|GetSpawn%20Chance) (Variables|Default|GetRandomStream))
      (Components|InstancedStaticMesh|AddInstance (Utilities|GetRandomHISM (Variables|Default|GetHISM%20Array) (Variables|Default|GetHISM%20Array%20Length) (Variables|Default|GetRandomStream)) (Math|Transform|MakeTransform (Utilities|AddRandomLocation (Utilities|AddVerticalLocation (Spline|GetLocationatDistanceAlongSpline _spline (* _index (Variables|Placement|GetSpacing)) "Local") (Variables|Default|GetAdd%20Vertical%20Offset)) (Variables|Placement|GetAdd%20Random%20Location) (Variables|Default|GetRandomStream)) (Utilities|AddRandomRotation (Utilities|AddMeshRotation (select (Variables|Placement|GetCustom%20Rotation) (Utilities|AddCustomRotation (Transformation|GetWorldRotation _spline) (Variables|Placement|GetAdd%20Custom%20Rotation)) (select (Variables|Default|GetVerticalAlignSplinePoints) (Spline|GetRotationatDistanceAlongSpline _spline (* _index (Variables|Placement|GetSpacing)) "Local") (Math|Rotator|MakeRotator 0.0 0.0 (.Yaw (Math|Rotator|BreakRotator (Spline|GetRotationatDistanceAlongSpline _spline (* _index (Variables|Placement|GetSpacing)) "Local")))))) (Variables|Default|GetAdd%20Mesh%20Yaw%20Rotation)) (Variables|Placement|GetAdd%20Random%20Rotation) (Variables|Default|GetRandomStream)) (Math|Vector|MakeVector _scale_output _scale_output _scale_output))))))