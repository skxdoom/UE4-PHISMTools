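; BP_PHISM_SplineMeshesBounds procedurally places instanced static meshes end to end along a spline, spaced by each mesh's bounds.
; The construction script repeatedly picks a random HISM and scale, using the scaled extent on the yaw-selected axis to advance along the spline, minus an overlap.
; Each instance follows spline yaw or full rotation, plus vertical and random offsets.
; Placement stops at the spline's end or the spawn limit.
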(event EventBeginPlay)

(event Collision|EventActorBeginOverlap
  (params (OtherActor :type Actor%20Object%20Reference)))

(event EventTick
  (params (DeltaSeconds :type Float%20%28single-precision%29)))

(fn ConstructionScript
  (|CallParentFunction)
  (CallFunction|SpawnInstancesbySpacing) ; Spawn Instances with user defined parameters
)

(fn SpawnInstancesbySpacing
  (bind _randomstream (Variables|Default|GetRandomStream))
  (bind _scale_min (Variables|Default|GetScale%20Min))
  (bind _scale_max (Variables|Default|GetScale%20Max))
  (bind _spline (Variables|Default|GetSpline))
  (bind _scale_output (Utilities|GetRandomScale _scale_min _scale_max _randomstream))
  (Utilities|FlowControl|ForLoopwithBreak 0 (Variables|Placement|GetMaxSpawns) :!label _label
    (:LoopBody
      ;[1 1 1] Defining temporal values
      (LocalVariables|SetInstanceTemp (Utilities|GetRandomHISM (Variables|Default|GetHISM%20Array) (Variables|Default|GetHISM%20Array%20Length) (Variables|Default|GetRandomStream)))
      (LocalVariables|SetInstanceScaleTemp (Math|Vector|MakeVector _scale_output _scale_output _scale_output))
      (LocalVariables|SetExtentCurrentTemp (Utilities|Select :Index (Variables|Default|GetAdd%20Mesh%20Yaw%20Rotation) :NewEnumerator0 (.X (Math|Vector|BreakVector (* (.boxextent (StaticMesh|GetBounds (Variables|/Script/Engine.StaticMeshComponent|GetStaticMesh (LocalVariables|GetInstanceTemp)))) (LocalVariables|GetInstanceScaleTemp)))) :NewEnumerator1 (.Y (Math|Vector|BreakVector (* (.boxextent (StaticMesh|GetBounds (Variables|/Script/Engine.StaticMeshComponent|GetStaticMesh (LocalVariables|GetInstanceTemp)))) (LocalVariables|GetInstanceScaleTemp)))) :NewEnumerator2 (.X (Math|Vector|BreakVector (* (.boxextent (StaticMesh|GetBounds (Variables|/Script/Engine.StaticMeshComponent|GetStaticMesh (LocalVariables|GetInstanceTemp)))) (LocalVariables|GetInstanceScaleTemp)))) :NewEnumerator3 (.Y (Math|Vector|BreakVector (* (.boxextent (StaticMesh|GetBounds (Variables|/Script/Engine.StaticMeshComponent|GetStaticMesh (LocalVariables|GetInstanceTemp)))) (LocalVariables|GetInstanceScaleTemp))))))
      ;[1 1 1] Breaking loop
      (if (< (+ (LocalVariables|GetDistanceTemp) (* (LocalVariables|GetExtentCurrentTemp) 2.0)) (Spline|GetSplineLength (Variables|Default|GetSpline)))
        ;[1 1 1] Spawning Instance
        (Components|InstancedStaticMesh|AddInstance (LocalVariables|GetInstanceTemp) (Math|Transform|MakeTransform (Utilities|AddRandomLocation (Utilities|AddVerticalLocation (Spline|GetLocationatDistanceAlongSpline _spline (+ (LocalVariables|GetDistanceTemp) (LocalVariables|GetExtentCurrentTemp)) "Local") (Variables|Default|GetAdd%20Vertical%20Offset)) (Variables|Placement|GetAdd%20Random%20Location) (Variables|Default|GetRandomStream)) (Utilities|AddRandomRotation (Utilities|AddMeshRotation (select (Variables|Default|GetVerticalAlignSplinePoints) (Spline|GetRotationatDistanceAlongSpline _spline (+ (LocalVariables|GetDistanceTemp) (LocalVariables|GetExtentCurrentTemp)) "Local") (Math|Rotator|MakeRotator 0.0 0.0 (.Yaw (Math|Rotator|BreakRotator (Spline|GetRotationatDistanceAlongSpline _spline (+ (LocalVariables|GetDistanceTemp) (LocalVariables|GetExtentCurrentTemp)) "Local"))))) (Variables|Default|GetAdd%20Mesh%20Yaw%20Rotation)) (Variables|Placement|GetAdd%20Random%20Rotation) (Variables|Default|GetRandomStream)) (LocalVariables|GetInstanceScaleTemp)))
        ;[1 1 1] Set distance along spline for next iterations
        (LocalVariables|SetDistanceTemp (+ (LocalVariables|GetDistanceTemp) (- (* (LocalVariables|GetExtentCurrentTemp) 2.0) (Variables|Placement|GetOverlapping%20Bounds))))
        (else
          (goto _label Break))))))