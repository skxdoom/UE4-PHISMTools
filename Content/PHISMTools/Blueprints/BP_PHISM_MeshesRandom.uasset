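; Placement actor that scatters random mesh instances inside a box or sphere volume, built in the construction script.
; It shows and sizes the volume for the chosen placement type, then for each Density step picks a random HISM and a random point from a random stream.
; A line trace decides whether each point can spawn and supplies location and alignment rotation, with optional pivot height compensation and vertical offset.
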(event EventBeginPlay)

(event Collision|EventActorBeginOverlap
  (params (OtherActor :type Actor%20Object%20Reference)))

(event EventTick
  (params (DeltaSeconds :type Float%20%28single-precision%29)))

(fn ConstructionScript
  (|CallParentFunction)
  (CallFunction|DefinePlacementStyle)
  (CallFunction|SpawnInstances))

(fn SpawnInstances
  (for _index (range 0 (- (Variables|Meshes|GetDensity) 1)) ; Repeat once for each mesh to spawn
    (CallFunction|SetInstanceTemporalValues (Utilities|GetRandomHISM (Variables|Default|GetHISM%20Array) (Variables|Default|GetHISM%20Array%20Length) (Variables|Default|GetRandomStream)))
    (bind (_location_output _align_rotation_output _canspawn) (CallFunction|LineTracingforPlacement (Utilities|Select :Index (Variables|Placement|GetPlacement%20Type) :NewEnumerator0 (Utilities|RandomPointinBox (Variables|Placement|GetBox%20Extent) (Variables|Default|GetRandomStream)) :NewEnumerator1 (Utilities|RandomPointinSphere (Variables|Placement|GetSphere%20Radius) (Variables|Default|GetRandomStream))) (Utilities|TraceDistance)))
    (if _canspawn
      ;[1 1 1] Spawn Instances
      (Components|InstancedStaticMesh|AddInstance (Variables|Default|GetInstance%20Temp) (Math|Transform|MakeTransform (Utilities|AddVerticalLocation (select (Variables|Default|GetPivot%20Point%20At%20Zero) _location_output (+ _location_output (Math|Vector|MakeVector 0.0 0.0 (.Z (Math|Vector|BreakVector (Variables|Default|GetInstance%20Box%20Extent%20Temp)))))) (Variables|Default|GetAdd%20Vertical%20Location)) _align_rotation_output (Variables|Default|GetInstance%20Scale%20Temp))))))

(fn DefinePlacementStyle
  (if (Utilities|Enum|Equal(Enum) (Variables|Placement|GetPlacement%20Type) "NewEnumerator0")
    (Rendering|SetVisibility (Variables|Default|GetBox) true false)
    (Rendering|SetVisibility (Variables|Default|GetSphere) false false)
    (Components|Box|SetBoxExtent (Variables|Default|GetBox) (Variables|Placement|GetBox%20Extent) true)
    (else
      (Rendering|SetVisibility (Variables|Default|GetSphere) true false)
      (Rendering|SetVisibility (Variables|Default|GetBox) false false)
      (Components|Sphere|SetSphereRadius (Variables|Default|GetSphere) (Variables|Placement|GetSphere%20Radius) true))))