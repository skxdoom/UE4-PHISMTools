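; BP_PHISM_Master is a base actor for PHISM tools that prepares Hierarchical Instanced Static Mesh components from a list of meshes.
; The construction script sets actor collision from a flag, then adds one HISM component per Meshes entry with shared cull distance and shadow settings.
; The components are stored in HISMArray for later use; this file adds no instances and has no active runtime logic.
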(event EventBeginPlay)

(event Collision|EventActorBeginOverlap
  (params (OtherActor :type Actor%20Object%20Reference)))

(event EventTick
  (params (DeltaSeconds :type Float%20%28single-precision%29)))

(fn ConstructionScript
  (CallFunction|SetCollisionEnabled)
  (CallFunction|DefineHISMArray))

(fn DefineHISMArray
  (bind _output_get (Variables|Default|SetHISM%20Array%20Length (Utilities|Array|Length (Variables|Meshes|GetMeshes))))
  (for _index (range 0 (- _output_get 1))
    (bind _returnvalue (AddComponent|AddHierarchicalInstancedStaticMeshComponent false)) ; Adding one HISM Component per one SM array item
    (Components|StaticMesh|SetStaticMesh _returnvalue (Utilities|Array|Get(acopy) (Variables|Meshes|GetMeshes) _index)) ; Setting SM to HISM Component
    ;[1 1 1] Optimization parameters
    (Components|InstancedStaticMesh|SetCullDistances _returnvalue (Variables|Optimization|GetStart%20Cull%20Distance) (Variables|Optimization|GetEnd%20Cull%20Distance))
    (Rendering|SetCastShadow _returnvalue (Variables|Optimization|GetCast%20Shadows))
    (Utilities|Array|Add (Variables|Default|GetHISM%20Array) _returnvalue) ; Array of HISM objects to operate with
  )
  (return))

(fn SetCollisionEnabled
  (Collision|SetActorEnableCollision (Variables|Meshes|GetEnable%20Collision)))