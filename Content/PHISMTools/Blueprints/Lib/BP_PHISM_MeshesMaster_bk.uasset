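; Master Blueprint for the PHISM mesh tools, providing placement tracing that decides whether a mesh can spawn at a given local-space point.
; TracingForPlacement sphere-traces WorldStatic objects, rejecting initial overlaps and, with vertical snap, requiring a hit below.
; It returns a local-space location and rotation with optional normal alignment and seeded random yaw.
; Debug helpers draw the collision radius and a green or red line showing spawn validity.
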(event EventBeginPlay
  (|CallParentFunction) ; This node is disabled and will not be called.\nDrag off pins to build functionality.
)

(event Collision|EventActorBeginOverlap
  (params (OtherActor :type Actor%20Object%20Reference))
  (|CallParentFunction OtherActor) ; This node is disabled and will not be called.\nDrag off pins to build functionality.
)

(event EventTick
  (params (DeltaSeconds :type Float%20%28single-precision%29))
  (|CallParentFunction DeltaSeconds) ; This node is disabled and will not be called.\nDrag off pins to build functionality.
)

(fn ConstructionScript
  (|CallParentFunction))

(fn TracingforPlacement
  (params (Location%20Input :type Vector) (Tracing :type Float%20%28single-precision%29))
  (bind _returnvalue (Transformation|GetActorRotation))
  (bind _returnvalue_2 (Transformation|GetActorLocation))
  (bind _returnvalue_3 (Transformation|GetActorTransform))
  (bind (_x _y _z) (Math|Vector|BreakVector Location%20Input))
  (bind _randomstream (Variables|Default|GetRandomStream))
  (bind _vertical_snap (Variables|Placement|GetVertical%20Snap))
  (bind _returnvalue_4 (Math|Vector|GetUpVector _returnvalue))
  (bind _returnvalue_5 (Math|Vector|MakeVector _x _y _z))
  (bind _returnvalue_6 (Math|Random|RandomFloatinRangefromStream 0.0 3.6e+02 _randomstream))
  (bind _returnvalue_7 (select _vertical_snap Location%20Input _returnvalue_5))
  (bind _returnvalue_8 (Math|Vector|RotateVector _returnvalue_7 _returnvalue))
  (bind _returnvalue_9 (+ _returnvalue_4 _returnvalue_8))
  (bind _returnvalue_10 (+ _returnvalue_2 _returnvalue_9))
  (bind (_x_2 _y_2 _z_2) (Math|Vector|BreakVector _returnvalue_10))
  ;[1 1 1] Sphere Tracing
  (bind (_outhit _returnvalue_11) (Collision|SphereTraceForObjects _returnvalue_10 (select (Variables|Placement|GetVertical%20Snap) (Math|Vector|MakeVector _x_2 _y_2 (- _z_2 Tracing)) _returnvalue_10) (Variables|Placement|GetCollision%20Tracing%20Radius) (Utilities|Array|MakeArray "ObjectTypeQuery1") false (Variables|Placement|GetActors%20To%20Ignore) "None" (Variables|Placement|GetIgnore%20Self%20Collision) "(R=1.000000,G=0.000000,B=0.000000,A=1.000000)" "(R=0.000000,G=1.000000,B=0.000000,A=1.000000)" 1.0))
  ;[1 1 1] Booleans controling spawn conditions
  (if (Variables|Placement|GetVertical%20Snap) ; Snapping
    (if (.bInitialOverlap (Collision|BreakHitResult _outhit)) ; Overlapping
      (Variables|Default|SetCan%20Spawn false)
      (elif _returnvalue_11 ; Hit
        (Variables|Default|SetCan%20Spawn true)
        (if true :!label _label ; Reserve
          _
          (else
            (Variables|Default|SetCan%20Spawn false)))
        (else
          (Variables|Default|SetCan%20Spawn false))))
    (elif (.bInitialOverlap (Collision|BreakHitResult _outhit)) ; Overlapping
      (Variables|Default|SetCan%20Spawn false)
      (else
        (Variables|Default|SetCan%20Spawn true)
        (goto _label))))
  (Debug|DrawPlacementLine (Variables|Default|GetCan%20Spawn))
  (return (Math|Transform|InverseTransformLocation _returnvalue_3 (select (Variables|Placement|GetVertical%20Snap) (.ImpactPoint (Collision|BreakHitResult _outhit)) (.TraceStart (Collision|BreakHitResult _outhit)))) (Math|Transform|InverseTransformRotation _returnvalue_3 (Math|Rotator|CombineRotators (select (Variables|Placement|GetVertical%20Anign) (Math|Rotator|MakeRotfromZ (.Normal (Collision|BreakHitResult _outhit))) "0, 0, 0") (Math|Rotator|SelectRotator (select (Variables|Placement|GetVertical%20Anign) (Math|Vector|RotatorfromAxisandAngle (.Normal (Collision|BreakHitResult _outhit)) _returnvalue_6) (Math|Rotator|MakeRotator 0.0 0.0 _returnvalue_6)) "0, 0, 0" (Variables|Placement|GetRandom%20Yaw)))) (Variables|Default|GetCan%20Spawn)))

(fn ShowCollisionRadius
  (Rendering|Debug|DrawDebugSphere (Transformation|GetActorLocation) (Variables|Placement|GetCollision%20Tracing%20Radius) 12 "(R=0.000000,G=1.000000,B=0.000000,A=1.000000)" 8.0))

(fn DrawPlacementLine
  (params (CanSpawn :type Boolean))
  (bind _returnvalue (Transformation|GetActorLocation))
  (bind _collision_tracing_distance (Variables|Placement|GetCollision%20Tracing%20Distance))
  (bind (_x _y _z) (Math|Vector|BreakVector _returnvalue))
  (bind _returnvalue_2 (- _z _collision_tracing_distance))
  (bind _returnvalue_3 (Math|Vector|MakeVector _x _y _returnvalue_2))
  (if CanSpawn
    (Rendering|Debug|DrawDebugLine _returnvalue _returnvalue_3 "(R=0.000000,G=1.000000,B=0.000000,A=1.000000)" 0.1 4.0)
    (else
      (Rendering|Debug|DrawDebugLine _returnvalue _returnvalue_3 "(R=1.000000,G=0.000000,B=0.000000,A=1.000000)" 0.1 4.0))))