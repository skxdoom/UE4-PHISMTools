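; BP_PHISM_SplineMaster is a spline actor, apparently a base for PHISM tools, that prepares its spline in the construction script.
; It applies the closed-loop setting, then optionally snaps every point except the first onto surfaces using vertical Visibility line traces within SnappingDistanceZ.
; Aligning point up vectors to hit normals and setting point types are present but disconnected, so neither takes effect.
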(event EventBeginPlay)

(event Collision|EventActorBeginOverlap
  (params (OtherActor :type Actor%20Object%20Reference)))

(event EventTick
  (params (DeltaSeconds :type Float%20%28single-precision%29)))

(fn ConstructionScript
  (|CallParentFunction)
  (CallFunction|SetClosedSpline (Variables|Default|GetSpline))
  (CallFunction|SplinePointVerticalSnap (Variables|Default|GetSpline)))

(fn SetClosedSpline
  (params (SplineComponent :type Spline%20Component%20Object%20Reference))
  (Spline|SetClosedLoop SplineComponent (Variables|Spline|GetClosedSpline) true))

(fn SplinePointVerticalSnap
  (params (Spline :type Spline%20Component%20Object%20Reference))
  (if (Variables|Spline|GetVerticalSnapSplinePoints)
    (for _index (range 1 (- (Spline|GetNumberOfSplinePoints Spline) 1)) ; Don't snap First point\nKeeping origin points okay
      (bind (_outhit _returnvalue) (Collision|LineTraceByChannel (+ (Spline|GetLocationatSplinePoint Spline _index "World") (Math|Vector|MakeVector 0.0 0.0 (Variables|Spline|GetSnappingDistanceZ))) (- (Spline|GetLocationatSplinePoint Spline _index "World") (Math|Vector|MakeVector 0.0 0.0 (Variables|Spline|GetSnappingDistanceZ))) "TraceTypeQuery1" false 0 "None"))
      (if _returnvalue
        (Spline|SetLocationatSplinePoint Spline _index (.Location (Collision|BreakHitResult _outhit)) "World" true)
        (if (Variables|Spline|GetVerticalAlignSplinePoints)
          _)))))

(fn SetPointType
  (params (Spline :type Spline%20Component%20Object%20Reference))
  (for _index (range 0 (- (Spline|GetNumberOfSplinePoints Spline) 2))
    (Spline|SetSplinePointType Spline _index (Variables|Spline|GetPointType) true)))