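; Spline-driven fence tool that places meshes along a spline in the construction script.
; It steps by scaled spacing, adding instances to HISMs picked via a random stream.
; Each faces the next sample point, optionally yaw-only, with yaw and vertical offsets.
; A separate static mesh caps the spline end, spawned only when a returned instance index equals the segment count, which multiple HISMs may prevent.
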(event EventBeginPlay)

(event Collision|EventActorBeginOverlap
  (params (OtherActor :type Actor%20Object%20Reference)))

(event EventTick
  (params (DeltaSeconds :type Float%20%28single-precision%29)))

(fn ConstructionScript
  (|CallParentFunction)
  (CallFunction|SpawnInstances) ; Spawn Instances with user defined parameters
)

(fn SpawnInstances
  (bind _spline (Variables|Default|GetSpline))
  (bind _scale (Variables|Meshes|GetScale))
  (bind _spline_2 (Variables|Default|GetSpline))
  (bind _spline_3 (Variables|Default|GetSpline))
  (bind _scale_2 (Variables|Meshes|GetScale))
  (bind _scale_3 (Variables|Meshes|GetScale))
  (bind _distancebetween (Variables|Placement|GetDistanceBetween))
  (bind _returnvalue (Spline|GetSplineLength _spline))
  (bind _returnvalue_2 (* _distancebetween _scale))
  (bind _returnvalue_3 (Math|Float|Division(WholeandRemainder) _returnvalue _returnvalue_2))
  (for _index (range 0 _returnvalue_3)
    ;[1 1 1] Spawning Instance
    (bind _returnvalue_4 (Components|InstancedStaticMesh|AddInstance (Utilities|GetRandomHISM (Variables|Default|GetHISM%20Array) (Variables|Default|GetHISM%20Array%20Length) (Variables|Default|GetRandomStream)) (Math|Transform|MakeTransform (Utilities|AddVerticalLocation (Spline|GetLocationatDistanceAlongSpline _spline_2 (* _index _returnvalue_2) "Local") (Variables|Default|GetAdd%20Vertical%20Offset)) (Utilities|AddMeshRotation (select (Variables|Default|GetVerticalAlignSplinePoints) (Math|Rotator|FindLookatRotation (Spline|GetLocationatDistanceAlongSpline _spline_2 (* _index _returnvalue_2) "Local") (Spline|GetLocationatDistanceAlongSpline _spline_2 (+ (* _index _returnvalue_2) _returnvalue_2) "Local")) (Math|Rotator|MakeRotator 0.0 0.0 (.Yaw (Math|Rotator|BreakRotator (Math|Rotator|FindLookatRotation (Spline|GetLocationatDistanceAlongSpline _spline_2 (* _index _returnvalue_2) "Local") (Spline|GetLocationatDistanceAlongSpline _spline_2 (+ (* _index _returnvalue_2) _returnvalue_2) "Local")))))) (Variables|Default|GetAdd%20Mesh%20Yaw%20Rotation)) (Math|Vector|MakeVector _scale_3 _scale_3 _scale_3))))
    ;[1 1 1] Spawning Last Mesh
    (if (== _returnvalue_4 _returnvalue_3) ; If it's the last instance on spline
      (bind _returnvalue_5 (AddComponent|AddStaticMeshComponent false (Math|Transform|MakeTransform (Utilities|AddVerticalLocation (Spline|GetLocationatSplinePoint _spline_3 (Spline|GetNumberOfSplinePoints _spline_3) "Local") (Variables|Default|GetAdd%20Vertical%20Offset)) (Utilities|AddMeshRotation (select (Variables|Default|GetVerticalAlignSplinePoints) (Math|Rotator|FindLookatRotation (Spline|GetLocationatDistanceAlongSpline _spline_2 (* _index _returnvalue_2) "Local") (Spline|GetLocationatDistanceAlongSpline _spline_2 (+ (* _index _returnvalue_2) _returnvalue_2) "Local")) (Math|Rotator|MakeRotator 0.0 0.0 (.Yaw (Math|Rotator|BreakRotator (Math|Rotator|FindLookatRotation (Spline|GetLocationatDistanceAlongSpline _spline_2 (* _index _returnvalue_2) "Local") (Spline|GetLocationatDistanceAlongSpline _spline_2 (+ (* _index _returnvalue_2) _returnvalue_2) "Local")))))) (Variables|Default|GetAdd%20Mesh%20Yaw%20Rotation)) (Math|Vector|MakeVector _scale_2 _scale_2 _scale_2))))
      (Components|StaticMesh|SetStaticMesh _returnvalue_5 (Variables|Meshes|GetLastMesh)))))